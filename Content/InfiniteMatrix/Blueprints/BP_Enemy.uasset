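; BP_Enemy is a short-lived spinning cube enemy that damages the player on contact and dies to lasers.
; It starts tiny with a three-second lifespan, and Tick rotates it while driving frame-based scale animations for spawning and death, each ending with a sound.
; A laser overlap sets Dying, which shrinks the cube until destroyed, while hitting BP_Player calls DecreaseHealth and destroys it immediately.
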(event OnComponentBeginOverlap(Cube)
  (params (OverlappedComponent :type Primitive%20Component%20Object%20Reference) (OtherActor :type Actor%20Object%20Reference) (OtherComp :type Primitive%20Component%20Object%20Reference) (OtherBodyIndex :type Integer) (bFromSweep :type Boolean) (SweepResult :type Hit%20Result%20Structure%20%28by%20ref%29))
  (Utilities|Casting|CastToBP_Laser OtherActor)
  (Variables|Default|SetDying true))

(event OnComponentHit(Cube)
  (params (HitComponent :type Primitive%20Component%20Object%20Reference) (OtherActor :type Actor%20Object%20Reference) (OtherComp :type Primitive%20Component%20Object%20Reference) (NormalImpulse :type Vector :default "0, 0, 0") (Hit :type Hit%20Result%20Structure%20%28by%20ref%29))
  (bind _asbp_player (Utilities|Casting|CastToBP_Player OtherActor))
  (Default|DecreaseHealth _asbp_player)
  (Actor|DestroyActor))

(event EventBeginPlay
  (Actor|SetLifeSpan 3.0)
  (Transformation|SetActorScale3D "0.100000,0.100000,0.100000"))

(event Collision|EventActorBeginOverlap
  (params (OtherActor :type Actor%20Object%20Reference)))

(event EventTick
  (params (DeltaSeconds :type Float%20%28single-precision%29))
  (Utilities|IsValid (Variables|Default|GetCube)
    (:Is%20Valid
      (Class|Actor|AddActorWorldRotation (Math|Rotator|MakeRotator 0.0 (* DeltaSeconds 2.5e+02) 0.0))
      (if (Variables|Default|GetDying)
        (CallFunction|StartDeath)
        (elif (Variables|Default|GetSpawning)
          (CallFunction|StartSpawn))))))

(fn ConstructionScript)

(fn StartDeath
  (bind _returnvalue (Transformation|GetActorScale3D))
  (if (> (.X (Math|Vector|BreakVector _returnvalue)) 0.0)
    (Transformation|SetActorScale3D (- _returnvalue 0.1))
    (else
      (Actor|DestroyActor)
      (Audio|PlaySoundatLocation "/Engine/VREditor/Sounds/UI/Camera_Shutter.Camera_Shutter" (Transformation|GetActorLocation) "0, 0, 0" 0.5 1.0 0.0 0 0 0))))

(fn StartSpawn
  (bind _returnvalue (Transformation|GetActorScale3D))
  (if (< (.X (Math|Vector|BreakVector _returnvalue)) 1.0)
    (Transformation|SetActorScale3D (+ _returnvalue 0.025))
    (else
      (Variables|Default|SetSpawning false)
      (Audio|PlaySoundatLocation "/Engine/VREditor/Sounds/UI/Laser_Pull.Laser_Pull" (Transformation|GetActorLocation) "0, 0, 0" 1.0 0.5 0.0 0 0 0))))