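; BP_Tunnel is a tunnel segment with a rotating holed wall that penalizes the player's score and health on end overlap and destroys other actors.
; Its trigger zone has the player spawn pickups and enemies and gain score, requests another tunnel from TunnelSpawner, then destroys the segment.
; RandomizeWall varies hole mesh and roll.
; UpdateColor tints every tunnel's dynamic materials red, yellow or green by player health.
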(event OnComponentBeginOverlap(TriggerZone)
  (params (OverlappedComponent :type Primitive%20Component%20Object%20Reference) (OtherActor :type Actor%20Object%20Reference) (OtherComp :type Primitive%20Component%20Object%20Reference) (OtherBodyIndex :type Integer) (bFromSweep :type Boolean) (SweepResult :type Hit%20Result%20Structure%20%28by%20ref%29))
  (bind _asbp_player (Utilities|Casting|CastToBP_Player OtherActor))
  (Default|SpawnHealthPack _asbp_player)
  (Default|SpawnEnemy _asbp_player)
  (Default|IncreaseScore _asbp_player)
  (Default|SpawnTunnelatSpawnPoint (Variables|Default|GetTunnelSpawner))
  (Actor|DestroyActor))

(event OnComponentEndOverlap(WallMesh)
  (params (OverlappedComponent :type Primitive%20Component%20Object%20Reference) (OtherActor :type Actor%20Object%20Reference) (OtherComp :type Primitive%20Component%20Object%20Reference) (OtherBodyIndex :type Integer))
  (bind _asbp_player (Utilities|Casting|CastToBP_Player OtherActor)
    (:then
      (Default|DecreaseScore _asbp_player)
      (Default|DecreaseHealth _asbp_player))
    (:CastFailed
      (Actor|DestroyActor OtherActor))))

(event EventBeginPlay
  (bind _wallmesh (Variables|Default|GetWallMesh))
  (bind _returnvalue (Rendering|Material|CreateDynamicMaterialInstance (Variables|Debug|GetStaticMeshComponent) 0 "/Game/InfiniteMatrix/Materials/MI_Tunnel.MI_Tunnel" "None" :!class /Script/Engine.PrimitiveComponent))
  (Variables|Default|SetMI _returnvalue)
  (Rendering|Material|SetMaterial (Variables|Debug|GetStaticMeshComponent) 0 _returnvalue)
  (bind _returnvalue_2 (Rendering|Material|CreateDynamicMaterialInstance _wallmesh 0 "/Game/InfiniteMatrix/Materials/MI_Hole.MI_Hole" "None" :!class /Script/Engine.PrimitiveComponent))
  (Variables|Default|SetMI2 _returnvalue_2)
  (Rendering|Material|SetMaterial _wallmesh 0 _returnvalue_2)
  (CallFunction|UpdateColor))

(event EventTick
  (params (DeltaSeconds :type Float%20%28single-precision%29))
  (Transformation|AddLocalRotation (Variables|Default|GetWallMesh) (Math|Rotator|MakeRotator (* DeltaSeconds (Variables|Default|GetRotateSpeed)) 0.0 0.0) false false))

(fn ConstructionScript)

(fn RandomizeWall
  (Components|StaticMesh|SetStaticMesh (Variables|Default|GetWallMesh) (Utilities|Select :Index (Math|Random|RandomIntegerinRange 0 3) :Option%200 "/Game/InfiniteMatrix/Meshes/SM_Hole_01.SM_Hole_01" :Option%201 "/Game/InfiniteMatrix/Meshes/SM_Hole_02.SM_Hole_02" :Option%202 "/Game/InfiniteMatrix/Meshes/SM_Hole_03.SM_Hole_03" :Option%203 "/Game/InfiniteMatrix/Meshes/SM_Hole_04.SM_Hole_04"))
  (Transformation|AddLocalRotation (Variables|Default|GetWallMesh) (Math|Rotator|MakeRotator (Math|Random|RandomFloatinRange 0.0 3.6e+02) 0.0 0.0) false false))

(fn UpdateColor
  (bind _redtext (Variables|Default|GetRedText))
  (bind _yellowtext (Variables|Default|GetYellowText))
  (bind _greentext (Variables|Default|GetGreenText))
  (bind _returnvalue (Actor|GetActorOfClass "/Game/InfiniteMatrix/Blueprints/BP_Player.BP_Player_C"))
  (bind _outactors (Actor|GetAllActorsOfClass "BP_Tunnel_C"))
  (for _array_element _outactors
    (switch int (Variables|/Game/InfiniteMatrix/Blueprints/BP_Player.BP_Player_C|GetPlayerHealth _returnvalue)
      (:1
        (Rendering|Material|SetVectorParameterValue (Variables|BP_Tunnel_C|GetMI _array_element) "TextColor" _redtext :!class /Script/Engine.MaterialInstanceDynamic)
        (Rendering|Material|SetVectorParameterValue (Variables|BP_Tunnel_C|GetMI _array_element) "BackgroundColor" (Variables|Default|GetRedBackground) :!class /Script/Engine.MaterialInstanceDynamic)
        (Rendering|Material|SetVectorParameterValue (Variables|BP_Tunnel_C|GetMI2 _array_element) "Color" _redtext :!class /Script/Engine.MaterialInstanceDynamic))
      (:2
        (Rendering|Material|SetVectorParameterValue (Variables|BP_Tunnel_C|GetMI _array_element) "TextColor" _yellowtext :!class /Script/Engine.MaterialInstanceDynamic)
        (Rendering|Material|SetVectorParameterValue (Variables|BP_Tunnel_C|GetMI _array_element) "BackgroundColor" (Variables|Default|GetYellowBackground) :!class /Script/Engine.MaterialInstanceDynamic)
        (Rendering|Material|SetVectorParameterValue (Variables|BP_Tunnel_C|GetMI2 _array_element) "Color" _yellowtext :!class /Script/Engine.MaterialInstanceDynamic))
      (:3
        (Rendering|Material|SetVectorParameterValue (Variables|BP_Tunnel_C|GetMI _array_element) "TextColor" _greentext :!class /Script/Engine.MaterialInstanceDynamic)
        (Rendering|Material|SetVectorParameterValue (Variables|BP_Tunnel_C|GetMI _array_element) "BackgroundColor" (Variables|Default|GetGreenBackground) :!class /Script/Engine.MaterialInstanceDynamic)
        (Rendering|Material|SetVectorParameterValue (Variables|BP_Tunnel_C|GetMI2 _array_element) "Color" _greentext :!class /Script/Engine.MaterialInstanceDynamic)))))