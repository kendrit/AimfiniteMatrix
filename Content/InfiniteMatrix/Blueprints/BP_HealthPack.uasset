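; BP_HealthPack is a short-lived health pickup actor for BP_Player that expires three seconds after spawning.
; Tick spins the Cube component around yaw at a frame-rate-independent speed.
; When a BP_Player hits the Cube, it calls IncreaseHealth on that player, destroys itself and plays a 2D camera shutter sound; pickup relies on component hit events, as the overlap event is disabled.
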(event OnComponentHit(Cube)
  (params (HitComponent :type Primitive%20Component%20Object%20Reference) (OtherActor :type Actor%20Object%20Reference) (OtherComp :type Primitive%20Component%20Object%20Reference) (NormalImpulse :type Vector :default "0, 0, 0") (Hit :type Hit%20Result%20Structure%20%28by%20ref%29))
  (bind _asbp_player (Utilities|Casting|CastToBP_Player OtherActor))
  (Default|IncreaseHealth _asbp_player)
  (Actor|DestroyActor)
  (Audio|PlaySound2D "/Engine/VREditor/Sounds/UI/Camera_Shutter.Camera_Shutter" 1.0 1.0 0.0 0 0))

(event EventBeginPlay
  (Actor|SetLifeSpan 3.0))

(event Collision|EventActorBeginOverlap
  (params (OtherActor :type Actor%20Object%20Reference)))

(event EventTick
  (params (DeltaSeconds :type Float%20%28single-precision%29))
  (bind _cube (Variables|Default|GetCube))
  (Utilities|IsValid _cube
    (:Is%20Valid
      (Transformation|AddWorldRotation _cube (Math|Rotator|MakeRotator 0.0 0.0 (* DeltaSeconds 2.5e+02)) false false))))

(fn ConstructionScript)