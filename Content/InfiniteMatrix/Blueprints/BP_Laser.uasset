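; BP_Laser is a projectile that awards score to the player who fired it when it hits an enemy.
; Tick moves it along world X at BulletVelocity with sweep, regardless of its rotation, and it expires after a few seconds.
; Overlapping a BP_Enemy calls IncreaseScore on the BP_Player instigator, then removes the laser through a near-zero lifespan; the enemy is left untouched here.
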(event EventBeginPlay
  (Actor|SetLifeSpan 3.0))

(event Collision|EventActorBeginOverlap
  (params (OtherActor :type Actor%20Object%20Reference))
  (Utilities|Casting|CastToBP_Enemy OtherActor)
  (bind _asbp_player (Utilities|Casting|CastToBP_Player (Variables|Actor|GetInstigator)))
  (Default|IncreaseScore _asbp_player)
  (Actor|SetLifeSpan 0.0001))

(event EventTick
  (params (DeltaSeconds :type Float%20%28single-precision%29))
  (Transformation|AddActorWorldOffset (Math|Vector|MakeVector (* DeltaSeconds (Variables|Default|GetBulletVelocity)) 0.0 0.0) true))

(fn ConstructionScript)